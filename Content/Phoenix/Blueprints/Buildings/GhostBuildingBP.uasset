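; Placement ghost for build mode that previews a building on a grid-snapped cursor position and packages it as a construction struct.
; ConstructBuilding briefly spawns the building class to read its mesh and proxy, then activates the ghost.
; Tick flags actor overlaps, otherwise line-traces corners and center for excessive slope and box-traces to set ground height.
; Either failure swaps in the error material and sets the status exposed by GetOverlappingStatus.
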(event `OnSpawn`
  (params (DisplayMesh :type "StaticMesh Object Reference") (BuildingClass :type "/Game/Phoenix/Blueprints/Buildings/BuildingMasterBP Class Reference") (ConstructionProxy :type "/Game/Phoenix/Blueprints/Construction/ConstructionProxyBP Class Reference"))
  ;[1 1 1] Spawn
  (if (not (`self.IsActive`))
    (set `self.BuildingClass` BuildingClass)
    (set `self.ConstructionProxy` ConstructionProxy)
    (set `self.DisplayMesh` DisplayMesh)
    (set `self.IsActive` true)
    (set `/Game/Phoenix/Blueprints/CameraPawnController.BuildModeActive` true (`self.ControllerRef`))
    (`StaticMeshComponent.SetStaticMesh` (`self.GhostBuildingMesh`) (`self.DisplayMesh`))
    (`self.OpenTickGate`)
    (`self.SetMaterial` (not (`self.IsOverlapping`)))
    (set `self.Extent` (`.BoxExtent` (`KismetSystemLibrary.GetComponentBounds` (`self.GhostBuildingMesh`))))))

(event `KillGhost`
  ;[1 1 1] KillGhost
  (set `self.BuildingClass` null)
  (set `self.ConstructionProxy` null)
  (set `self.DisplayMesh` null)
  (set `self.IsActive` false)
  (set `/Game/Phoenix/Blueprints/CameraPawnController.BuildModeActive` false (`self.ControllerRef`))
  (`StaticMeshComponent.SetStaticMesh` (`self.GhostBuildingMesh`) (`self.DisplayMesh`))
  (`self.K2_SetActorRotation` (struct)))

(event `/Game/Phoenix/Interfaces/I_HUD.ConstructBuilding`
  (params (mainBuilding :type "/Game/Phoenix/Blueprints/Buildings/BuildingMasterBP Class Reference"))
  ;[1 1 1] Construct Building
  (bind _returnvalue (`|SpawnActorFromClass` mainBuilding (`KismetMathLibrary.MakeTransform` (0.0 0.0 0.0)) "Undefined" "OverrideRootScale" null (`self.ControllerRef`) null))
  (`|ExecutionSequence`
    (:`then_0`
      (bind _asbuilding_master_bp (castclass `/Game/Phoenix/Blueprints/Buildings/BuildingMasterBP` mainBuilding))
      (`self.KillGhost`)
      (`self.OnSpawn` (`/Game/Phoenix/Blueprints/Buildings/BuildingMasterBP.DisplayMesh` _returnvalue) _asbuilding_master_bp (`/Game/Phoenix/Blueprints/Buildings/BuildingMasterBP.ConstructionProxy` _returnvalue)))
    (:`then_1`
      (`self.K2_DestroyActor` _returnvalue))))

(event `self.ReceiveTick`
  (params (DeltaSeconds :type "Float (single-precision)"))
  ;[1 1 1] Tick
  (`/Engine/EditorBlueprintResources/StandardMacros.Gate` true :!label _label
    (:`Exit`
      (`self.K2_SetActorLocation` self (`self.SetGridSnapVector`) false false)
      (if (`self.CheckOverlap`)
        (`self.SetMaterial` true)
        (else
          (bind _isvalidlocation (`self.CalculateSlope`))
          (`self.SetMaterial` _isvalidlocation))))))

(event `OpenTickGate`
  ;[1 1 1] Tick
  (goto _label :!via `Open`))

(event `CloseTickGate`
  ;[1 1 1] Tick
  (goto _label :!via `Close`))

(event `SetMaterial`
  (params (IsError :type Boolean))
  (bind _ghostbuildingmesh (`self.GhostBuildingMesh`))
  ;[1 1 1] SetMaterial
  (if (not (== IsError (`self.IsOverlapping`)))
    (bind _output_get (set `self.IsOverlapping` IsError))
    (if _output_get
      (`PrimitiveComponent.SetMaterial` _ghostbuildingmesh 0 "/Game/Materials/GhostErrorInstance.GhostErrorInstance")
      (else
        (`PrimitiveComponent.SetMaterial` _ghostbuildingmesh 0 "/Game/Materials/GhostMaterialInstance.GhostMaterialInstance")))))

(fn `CalculateSlope`
  (returns (IsValidLocation :type Boolean))
  (locals (SlopeDifferences :type "Array of Float (double-precision)") (MaxDifferences :type "Float (double-precision)" :default 20.0))
  (bind (_actorlocation _forwardvector _rightvector) (`self.GetVectors`))
  (bind _actorlocation_2 (`self.GetVectors`))
  (bind (_actorlocation_3 _forwardvector_2 _rightvector_2) (`self.GetVectors`))
  (bind _actorlocation_4 (`self.GetVectors`))
  (bind (_actorlocation_5 _forwardvector_3 _rightvector_3) (`self.GetVectors`))
  (bind (_actorlocation_6 _forwardvector_4 _rightvector_4) (`self.GetVectors`))
  (bind (_extent_x _extent_y) (`KismetMathLibrary.BreakVector` (`self.Extent`)))
  (bind _maxdifferences (`local.MaxDifferences`))
  (bind _slopedifferences (`local.SlopeDifferences`))
  (bind (_indexofminvalue _minvalue) (`KismetMathLibrary.MinOfFloatArray` _slopedifferences))
  (bind (_indexofmaxvalue _maxvalue) (`KismetMathLibrary.MaxOfFloatArray` _slopedifferences))
  (`|ExecutionSequence`
    (:`then_0`
      (`|ExecutionSequence`
        (:`then_0`
          (bind _difference (`self.SlopeTrace` (+ _actorlocation_3 (* (+ _forwardvector_2 _rightvector_2) (`self.Extent`)))))
          (`KismetArrayLibrary.Array_Add` (`local.SlopeDifferences`) _difference))
        (:`then_1`
          (bind _difference_2 (`self.SlopeTrace` (+ _actorlocation_5 (* (+ (* _forwardvector_3 -1.0) _rightvector_3) (`self.Extent`)))))
          (`KismetArrayLibrary.Array_Add` (`local.SlopeDifferences`) _difference_2))
        (:`then_2`
          (bind _difference_3 (`self.SlopeTrace` (+ _actorlocation_6 (* (+ _forwardvector_4 (* _rightvector_4 -1.0)) (`self.Extent`)))))
          (`KismetArrayLibrary.Array_Add` (`local.SlopeDifferences`) _difference_3))
        (:`then_3`
          (bind _difference_4 (`self.SlopeTrace` (+ _actorlocation (* (+ (* _forwardvector -1.0) (* _rightvector -1.0)) (`self.Extent`)))))
          (`KismetArrayLibrary.Array_Add` (`local.SlopeDifferences`) _difference_4))
        (:`then_4`
          (bind _difference_5 (`self.SlopeTrace` (`self.GetVectors`)))
          (`KismetArrayLibrary.Array_Add` (`local.SlopeDifferences`) _difference_5))))
    (:`then_1`
      (if (and (> _indexofminvalue -1) (> _indexofmaxvalue -1))
        (bind (_outhit _returnvalue) (`KismetSystemLibrary.BoxTraceSingle` (+ _actorlocation_2 (0.0 0.0 1000.0)) (- _actorlocation_2 (0.0 0.0 1000.0)) (`KismetMathLibrary.MakeVector` _extent_x _extent_y 1.0) (struct) "TraceTypeQuery3"))
        (if _returnvalue
          (`self.K2_SetActorLocation` (`KismetMathLibrary.MakeVector` (.x _actorlocation_4) (.y _actorlocation_4) (.z (`.ImpactPoint` (`GameplayStatics.BreakHitResult` _outhit))))))))
    (:`then_2`
      (return (or (> (`KismetMathLibrary.Abs` _minvalue) _maxdifferences) (> (`KismetMathLibrary.Abs` _maxvalue) _maxdifferences))))))

(fn `CheckOverlap`
  (returns (IsOverlapping :type Boolean))
  (return (> (`KismetArrayLibrary.Array_Length` (`self.GetOverlappingActors` "/Script/Engine.Actor")) 0)))

(fn `GetConstructionStruct`
  (returns (ConstructionStruct :type "/Game/Structs/ConstructionStruct Structure"))
  (return (make `/Game/Structs/ConstructionStruct` (`self.BuildingClass`) (`self.ConstructionProxy`) (`KismetMathLibrary.MakeTransform` (`self.K2_GetActorLocation`) (`self.K2_GetActorRotation`)) (`self.DisplayMesh`) 1.0)))

(fn `GetOverlappingStatus`
  (returns (IsOverlapping :type Boolean))
  (return (`self.IsOverlapping`)))

(fn `GetVectors`
  (returns (ActorLocation :type "Vector Structure") (ForwardVector :type "Vector Structure") (RightVector :type "Vector Structure"))
  (bind _returnvalue (`self.K2_GetActorRotation`))
  (return (`self.K2_GetActorLocation`) (`KismetMathLibrary.GetForwardVector` _returnvalue) (`KismetMathLibrary.GetRightVector` _returnvalue)))

(fn `SetCalendar`
  (params (Date :type "Array of Integer (by ref)"))
  (returns (Success :type Boolean))
  (return false))

(fn `SetClock`
  (params (Time :type "Array of Integer (by ref)"))
  (returns (Success :type Boolean))
  (return false))

(fn `SetCursorPosition`
  (params (CursorLocation :type "Vector Structure"))
  (set `self.CursorWorldPosition` CursorLocation)
  (return))

(fn `SetGridSnapVector`
  (returns (GridSnap :type "Vector Structure"))
  (bind (_cursorworldposition_x _cursorworldposition_y _cursorworldposition_z) (`KismetMathLibrary.BreakVector` (`self.CursorWorldPosition`)))
  (bind _gridsize (`self.GridSize`))
  (return (`KismetMathLibrary.MakeVector` (`/Game/Library/FunctionLibrary.GridSnap` _cursorworldposition_x _gridsize) (`/Game/Library/FunctionLibrary.GridSnap` _cursorworldposition_y _gridsize) (`/Game/Library/FunctionLibrary.GridSnap` _cursorworldposition_z _gridsize))))

(fn `SlopeTrace`
  (params (TraceLocation :type "Vector Structure"))
  (returns (Difference :type "Float (double-precision)"))
  (bind (_returnvalue_x _returnvalue_y _returnvalue_z) (`KismetMathLibrary.BreakVector` (`self.K2_GetActorLocation`)))
  (bind _outhit (`KismetSystemLibrary.LineTraceSingle` (+ TraceLocation (0.0 0.0 1000.0)) (- TraceLocation (0.0 0.0 1000.0)) "TraceTypeQuery3"))
  (return (- _returnvalue_z (.z (`.ImpactPoint` (`GameplayStatics.BreakHitResult` _outhit))))))

(fn `UserConstructionScript`)