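; CameraPawn is a camera pawn that keeps its height just above the surface beneath it.
; Each tick it line traces vertically from above itself down to world zero on TraceTypeQuery3.
; If the impact height is within an upper limit, it moves to a small fixed offset above that point, keeping X and Y, without checking whether the trace hit.
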(event `self.ReceiveTick`
  (params (DeltaSeconds :type "Float (single-precision)"))
  (bind (_returnvalue_x _returnvalue_y _returnvalue_z) (`KismetMathLibrary.BreakVector` (`self.K2_GetActorLocation` self)))
  (bind (_returnvalue_x_2 _returnvalue_y_2) (`KismetMathLibrary.BreakVector` (`self.K2_GetActorLocation` self)))
  (bind (_returnvalue_x_3 _returnvalue_y_3) (`KismetMathLibrary.BreakVector` (`self.K2_GetActorLocation` self)))
  (bind _outhit (`KismetSystemLibrary.LineTraceSingle` (`KismetMathLibrary.MakeVector` _returnvalue_x _returnvalue_y (+ _returnvalue_z 1000.0)) (`KismetMathLibrary.MakeVector` _returnvalue_x_2 _returnvalue_y_2) "TraceTypeQuery3"))
  (bind (_bblockinghit _binitialoverlap _time _distance _location _impactpoint) (`GameplayStatics.BreakHitResult` _outhit))
  (if (<= (.z _impactpoint) 2500.0)
    (`self.K2_SetActorLocation` (`KismetMathLibrary.MakeVector` _returnvalue_x_3 _returnvalue_y_3 (+ (.z _impactpoint) 50.0)))))

(fn `UserConstructionScript`)